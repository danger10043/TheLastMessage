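; BP_BossGunMeshSequence is a boss gun mesh actor that can play a dissolve effect, apparently for use in sequences.
; BeginPlay creates a dynamic material instance for each GunMesh material slot, sets its Dissolve parameter to the starting value and caches it.
; The Dissolve event resets the cached instances and restarts a timeline, whose alpha lerps the parameter across all of them.
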(event Custom|Dissolve
  (for _array_element (Variables|Default|GetDissolveMIDs)
    (Rendering|Material|SetScalarParameterValue _array_element "Dissolve" -0.2 :!class /Script/Engine.MaterialInstanceDynamic)
    (bind _dissolvealpha (Timeline|타임라인 PlayFromStart)
      (:Update
        (for _array_element_2 (Variables|Default|GetDissolveMIDs)
          (Rendering|Material|SetScalarParameterValue _array_element_2 "Dissolve" (Math|Float|Lerp -0.2 1.5 _dissolvealpha) :!class /Script/Engine.MaterialInstanceDynamic))))))

(event EventBeginPlay
  (bind _gunmesh (Variables|Default|GetGunMesh))
  (bind _returnvalue (Rendering|Material|GetNumMaterials _gunmesh))
  (Utilities|Array|Clear (Variables|Default|GetDissolveMIDs))
  (if (> _returnvalue 0)
    (for _index (range 0 (- _returnvalue 1))
      (bind _returnvalue_2 (Rendering|Material|CreateDynamicMaterialInstance (Variables|Default|GetGunMesh) _index 0 "None" :!class /Script/Engine.PrimitiveComponent))
      (Utilities|IsValid _returnvalue_2
        (:Is%20Valid
          (Rendering|Material|SetScalarParameterValue _returnvalue_2 "Dissolve" -0.2 :!class /Script/Engine.MaterialInstanceDynamic)
          (Utilities|Array|Add (Variables|Default|GetDissolveMIDs) _returnvalue_2))))))

(fn ConstructionScript)