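; BP_InteractionComponent is a gimmick component that relays interaction queries and highlight changes to target objects.
; QueryCanInteract validates the target and interactor, then returns the target's CanInteractMessage result if it implements BPI_Interactable, otherwise false.
; SendHighlightMessage forwards a visibility flag to any valid target through SetInteractionHighlightMessage.
; It holds no detection logic, and its BeginPlay and Tick events are empty.
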(event EventBeginPlay)

(event EventTick
  (params (DeltaSeconds :type Float%20%28single-precision%29)))

(event EventSendHighlightMessage
  (params (Target :type Actor%20Object%20Reference) (bVisible :type Boolean))
  (Utilities|IsValid Target
    (:Is%20Valid
      (Class|BPIInteractable|SetInteractionHighlight(Message) Target bVisible))))

(fn QueryCanInteract
  (params (Target :type Actor%20Object%20Reference) (Interactor :type Actor%20Object%20Reference))
  (Utilities|IsValid Target
    (:Is%20Valid
      (Utilities|IsValid Interactor
        (:Is%20Valid
          (if (Utilities|DoesObjectImplementInterface Target "/Game/Main/Blueprints/Gimmick/BPI_Interactable.BPI_Interactable_C")
            (bind _bcaninteract (Class|BPIInteractable|CanInteract(Message) Target Interactor))
            (return _bcaninteract)
            (else
              (return false))))
        (:Is%20Not%20Valid
          (return false))))
    (:Is%20Not%20Valid
      (return false))))