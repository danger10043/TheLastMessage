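; BP_ExplosiveBomb is an explosive bomb gimmick in the push-pull set that players can interact with.
; The Blueprint is a thin forwarding layer, casting interactors to PlayerBase before calling PerformInteraction or CanInteractInternal.
; Highlight and active-state changes pass to UpdateInteractionHighlight and ApplyActiveState, and GetGimmickActive returns IsActive.
; The graphs hold no explosion or push-pull logic, and BeginPlay, overlap, Tick and construction are empty.
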(event EventBeginPlay)

(event Collision|EventActorBeginOverlap
  (params (OtherActor :type Actor%20Object%20Reference)))

(event EventTick
  (params (DeltaSeconds :type Float%20%28single-precision%29)))

(event EventInteract
  (params (Interactor :type Actor%20Object%20Reference))
  (bind _asplayer_base (Utilities|Casting|CastToPlayerBase Interactor))
  (Class|GimmickBase|PerformInteraction _asplayer_base))

(event EventSetInteractionHighlight
  (params (bVisible :type Boolean))
  (Class|GimmickBase|UpdateInteractionHighlight bVisible))

(event EventSetGimmickActive
  (params (bNewActive :type Boolean))
  (Class|GimmickBase|ApplyActiveState bNewActive))

(fn ConstructionScript)

(fn CanInteract
  (params (Interactor :type Actor%20Object%20Reference))
  (bind _asplayer_base (Utilities|Casting|CastToPlayerBase Interactor))
  (return (Class|GimmickBase|CanInteractInternal _asplayer_base)))

(fn GetGimmickActive
  (return (Variables|Default|GetbIsActive)))