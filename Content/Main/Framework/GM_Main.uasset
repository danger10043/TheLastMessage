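; GM_Main is a game mode Blueprint that switches background music between exploration and boss combat.
; On BeginPlay it starts both looping 2D tracks at once, keeps the boss track near silent, and starts a half-second polling timer.
; Each poll finds the BossMonster, tests the player against its TargetDetectionBox bounds and defeated flag, then crossfades the two tracks through volume adjustments rather than restarting them.
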(event EventBeginPlay
  (CallFunction|StartMusic))

(event EventTick
  (params (DeltaSeconds :type Float%20%28single-precision%29)))

(fn ConstructionScript)

(fn StartMusic
  (bind _returnvalue (Audio|SpawnSound2D "/Game/Main/Audio/Music/MUS_Exploration_Loop.MUS_Exploration_Loop" 1.0 1.0 0.0 0 false false))
  (Variables|Default|SetExplorationMusic _returnvalue)
  (bind _returnvalue_2 (Audio|SpawnSound2D "/Game/Main/Audio/Music/MUS_BossCombat_Loop.MUS_BossCombat_Loop" 1.0 1.0 0.0 0 false false))
  (bind _output_get (Variables|Default|SetBossMusic _returnvalue_2))
  (Audio|Components|Audio|AdjustVolume _output_get 0.0 0.001 "Linear" :!class /Script/Engine.AudioComponent)
  (Utilities|Time|SetTimerbyFunctionName 0 "TickBossMusic" 0.5 true))

(fn TickBossMusic
  (bind _returnvalue (Game|Player|GetPlayerPawn 0))
  (if (not (Utilities|IsValid (Variables|Default|GetMusicBoss)))
    (bind _returnvalue_2 (Actor|GetActorOfClass "/Script/TheLastMessage.BossMonster"))
    (Variables|Default|SetMusicBoss _returnvalue_2))
  (if (and (Utilities|IsValid (Variables|Default|GetMusicBoss)) (Utilities|IsValid _returnvalue))
    (if (Utilities|IsValid (Variables|/Script/TheLastMessage.BossMonster|GetTargetDetectionBox (Variables|Default|GetMusicBoss)))
      (Audio|Components|Audio|AdjustVolume (Variables|Default|GetExplorationMusic) 1.5 (Math|Float|SelectFloat 1.0 0.001 (not (and (Math|Geometry|IsPointinBox (Transformation|GetActorLocation _returnvalue) (.Origin (Collision|GetActorBounds (Variables|/Script/TheLastMessage.BossMonster|GetTargetDetectionBox (Variables|Default|GetMusicBoss)) false false)) (.BoxExtent (Collision|GetActorBounds (Variables|/Script/TheLastMessage.BossMonster|GetTargetDetectionBox (Variables|Default|GetMusicBoss)) false false))) (not (Variables|/Script/TheLastMessage.BossMonster|GetbIsDefeated (Variables|Default|GetMusicBoss)))))) "Linear" :!class /Script/Engine.AudioComponent)
      (Audio|Components|Audio|AdjustVolume (Variables|Default|GetBossMusic) 1.5 (Math|Float|SelectFloat 1.0 0.001 (and (Math|Geometry|IsPointinBox (Transformation|GetActorLocation _returnvalue) (.Origin (Collision|GetActorBounds (Variables|/Script/TheLastMessage.BossMonster|GetTargetDetectionBox (Variables|Default|GetMusicBoss)) false false)) (.BoxExtent (Collision|GetActorBounds (Variables|/Script/TheLastMessage.BossMonster|GetTargetDetectionBox (Variables|Default|GetMusicBoss)) false false))) (not (Variables|/Script/TheLastMessage.BossMonster|GetbIsDefeated (Variables|Default|GetMusicBoss))))) "Linear" :!class /Script/Engine.AudioComponent))))