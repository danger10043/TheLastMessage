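; BP_LI20_GravityLogic links gimmicks in the LI20 gameplay map to the player's gravity state.
; Each Tick, it checks whether player 0's ability system component has the State.Gravity.Reversed tag.
; The entry door's active state mirrors that tag, while the restore plate is enabled only when gravity is reversed and the fuse socket is active.
; State is polled every frame rather than driven by events.
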(event EventTick
  (params (DeltaSeconds :type Float%20%28single-precision%29))
  (bind _returnvalue (Game|GetPlayerCharacter 0))
  (bind _returnvalue_2 (Ability|GetAbilitySystemComponent _returnvalue))
  (bind _returnvalue_3 (GameplayTags|HasMatchingGameplayTag _returnvalue_2 "(TagName=\"State.Gravity.Reversed\")"))
  (Utilities|IsValid _returnvalue
    (:Is%20Valid
      (Class|GimmickBase|ApplyActiveState (Variables|Default|GetEntryDoor) _returnvalue_3)
      (Class|GimmickBase|SetGimmickEnabled (Variables|Default|GetRestorePlate) (and _returnvalue_3 (Class|GimmickBase|IsGimmickActive (Variables|Default|GetFuseSocket)))))))

(fn ConstructionScript)