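; BP_TimedSwitchGroup is a switch gimmick that relays an active state to linked devices and rejects direct interaction.
; SetGimmickActive passes the new state to ApplyActiveState, and GetGimmickActive reports IsActive.
; NotifyLinkedDevices sends SetGimmickActiveMessage to each valid entry in LinkedDevices.
; CanInteract always returns false, and no timing or grouping logic appears in these graphs.
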(event EventBeginPlay)

(event Collision|EventActorBeginOverlap
  (params (OtherActor :type Actor%20Object%20Reference)))

(event EventTick
  (params (DeltaSeconds :type Float%20%28single-precision%29)))

(event EventSetGimmickActive
  (params (bNewActive :type Boolean))
  (Class|GimmickBase|ApplyActiveState bNewActive))

(event EventNotifyLinkedDevices
  (params (bNewActive :type Boolean))
  (for _array_element (Variables|Default|GetLinkedDevices)
    (Utilities|IsValid _array_element
      (:Is%20Valid
        (Class|BPIInteractable|SetGimmickActive(Message) _array_element bNewActive)))))

(fn ConstructionScript)

(fn CanInteract
  (params (Interactor :type Actor%20Object%20Reference))
  (return false))

(fn GetGimmickActive
  (return (Variables|Default|GetbIsActive)))